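; BP_PDCombatCharacter is a combat character that fires projectiles with switchable ammo types and shows a debug health readout.
; Number keys set the current ammo type to Fire, Healing, Water or Regular.
; Left mouse spawns a BP_PDProjectile just ahead of the camera along its aim, then assigns it that ammo type.
; A looping timer draws the current-to-max health ratio above the character, and debug prints report ammo selection and shots.
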(event Custom|UpdateHealthDebug
  (Rendering|Debug|DrawDebugString (+ (Math|Vector|MakeVector 0.0 0.0 2e+02) (Transformation|GetActorLocation)) (Utilities|String|ToString(Float) (/ (Class|PDCombatCharacter|GetHealthCurrent) (Class|PDCombatCharacter|GetHealthMax))) 0 "(R=0.430840,G=0.369315,B=1.000000,A=1.000000)" 0.5))

(event EventBeginPlay
  (Utilities|Time|SetTimerbyFunctionName 0 "UpdateHealthDebug" 0.2 true))

(event Collision|EventActorBeginOverlap
  (params (OtherActor :type Actor%20Object%20Reference)))

(event EventTick
  (params (DeltaSeconds :type Float%20%28single-precision%29)))

(event Input|KeyboardEvents|1
  (params (Key :type Key%20Structure :default "None"))
  (:Pressed
    (Variables|Default|SetCurrentAmmoType "Fire")
    (Development|PrintString "Fire")))

(event Input|KeyboardEvents|3
  (params (Key :type Key%20Structure :default "None"))
  (:Pressed
    (Variables|Default|SetCurrentAmmoType "Water")
    (Development|PrintString "Water")))

(event Input|KeyboardEvents|2
  (params (Key :type Key%20Structure :default "None"))
  (:Pressed
    (Variables|Default|SetCurrentAmmoType "Healing")
    (Development|PrintString "healing")))

(event Input|KeyboardEvents|4
  (params (Key :type Key%20Structure :default "None"))
  (:Pressed
    (Variables|Default|SetCurrentAmmoType "Regular")
    (Development|PrintString "Regular")))

(event Input|MouseEvents|LeftMouseButton
  (params (Key :type Key%20Structure :default "None"))
  (:Pressed
    (bind _returnvalue (Game|SpawnActorfromClass "/Game/MyBlueprints/BP_PDProjectile.BP_PDProjectile_C" (Math|Transform|MakeTransform (+ (* (Math|Vector|GetForwardVector (Variables|Default|GetCamera)) (Class|KismetSystemLibrary|MakeLiteralInteger 100)) (Transformation|GetWorldLocation (Variables|Default|GetCamera))) (Transformation|GetWorldRotation (Variables|Default|GetCamera))) "AlwaysSpawn" "MultiplyWithRoot" 0 0))
    (bind _asbp_pdprojectile (Utilities|Casting|CastToBP_PDProjectile _returnvalue))
    (bind _output_get (Variables|/Script/test_paradark.PDProjectile|SetAmmoType _asbp_pdprojectile (Variables|Default|GetCurrentAmmoType)))
    (Development|PrintString (Utilities|String|EnumtoString _output_get))))

(fn ConstructionScript)